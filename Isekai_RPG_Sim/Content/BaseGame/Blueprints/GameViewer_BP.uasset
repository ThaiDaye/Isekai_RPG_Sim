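; Player-controlled orthographic camera pawn for viewing, editing and debugging the tile world, with pan and zoom.
; Held inputs drive Gate/Delay loops that make GameManager advance time, spawn entities at an accelerating rate or paint tiles at the cursor.
; Once world generation completes, Tick converts view, cursor and eight surrounding points into zone/chunk/tile coordinates.
; It also prints chunk and entity stats and draws nav paths of entities under the cursor.
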(event `Key|SpaceBar`
  (params (Key :type "Key Structure"))
  ;[0.8135 0.2445 1] INPUTS
  (:`Pressed`
    (`|ExecutionSequence`
      (:`then_0`
        (goto _label :!via `Open`))
      (:`then_1`
        (`/Engine/EditorBlueprintResources/StandardMacros.Gate` true :!label _label
          (:`Exit`
            (`|ExecutionSequence`
              (:`then_0`
                (`/Game/BaseGame/Blueprints/GameManager_BP.ProgressTime` (`self.GameManager`)))
              (:`then_1`
                (`KismetSystemLibrary.Delay` 0.25)
                (goto _label))))))))
  (:`Released`
    (goto _label :!via `Close`)))

(event `Key|MiddleMouseButton`
  (params (Key :type "Key Structure"))
  ;[0.8135 0.2445 1] INPUTS
  (:`Pressed`
    (`|ExecutionSequence`
      (:`then_0`
        (goto _label_2 :!via `Open`))
      (:`then_1`
        (`/Engine/EditorBlueprintResources/StandardMacros.Gate` true :!label _label_2
          (:`Exit`
            (`|ExecutionSequence`
              (:`then_0`
                (`/Game/BaseGame/Blueprints/GameManager_BP.Create Entity At Cursor` (`self.GameManager`))
                (set `self._spawnWindup` (`KismetMathLibrary.FClamp` (- (`self._spawnWindup`) 0.01) 0.002 0.25)))
              (:`then_1`
                (`KismetSystemLibrary.Delay` (`self._spawnWindup`))
                (goto _label_2))))))))
  (:`Released`
    (set `self._spawnWindup` 0.25)
    (goto _label_2 :!via `Close`)))

(event `Key|LeftMouseButton`
  (params (Key :type "Key Structure"))
  ;[0.8135 0.2445 1] INPUTS
  (:`Pressed`
    (`|ExecutionSequence`
      (:`then_0`
        (goto _label_3 :!via `Open`))
      (:`then_1`
        (`/Engine/EditorBlueprintResources/StandardMacros.Gate` true :!label _label_3
          (:`Exit`
            (`|ExecutionSequence`
              (:`then_0`
                (`/Game/BaseGame/Blueprints/GameManager_BP.ChangeTile` (`self.GameManager`) (`self.WorldCoords_Cursor`) 0))
              (:`then_1`
                (`KismetSystemLibrary.DelayUntilNextTick`)
                (goto _label_3))))))))
  (:`Released`
    (goto _label_3 :!via `Close`)))

(event `Key|RightMouseButton`
  (params (Key :type "Key Structure"))
  ;[0.8135 0.2445 1] INPUTS
  (:`Pressed`
    (`|ExecutionSequence`
      (:`then_0`
        (goto _label_4 :!via `Open`))
      (:`then_1`
        (`/Engine/EditorBlueprintResources/StandardMacros.Gate` true :!label _label_4
          (:`Exit`
            (`|ExecutionSequence`
              (:`then_0`
                (`/Game/BaseGame/Blueprints/GameManager_BP.ChangeTile` (`self.GameManager`) (`self.WorldCoords_Cursor`) 1))
              (:`then_1`
                (`KismetSystemLibrary.DelayUntilNextTick`)
                (goto _label_4))))))))
  (:`Released`
    (goto _label_4 :!via `Close`)))

(event `self.ReceiveBeginPlay`
  ;[1 1 1] BEGIN
  (`self.Possess`))

(event `InputAxis|InputAxis_UpDown`
  (params (AxisValue :type "Float (single-precision)"))
  ;[0.2619 0.8901 1] move camera
  (`self.AddMovementInput` (1.0 0.0 0.0) AxisValue))

(event `Key|Z`
  (params (Key :type "Key Structure"))
  ;[0.2619 0.8901 1] zoom camera
  (:`Pressed`
    (set `self._zoom` (`self.DefaultZoom`))
    (`CameraComponent.SetOrthoWidth` (`self.Camera`) (`self._zoom`) :!label _label_5)))

(event `InputAxis|InputAxis_MouseWheel`
  (params (AxisValue :type "Float (single-precision)"))
  ;[0.2619 0.8901 1] zoom camera
  (set `self._zoom` (`KismetMathLibrary.FClamp` (+ (* AxisValue (`self.CameraZoomSpeed`)) (`self._zoom`)) 512.0 524288.0))
  (goto _label_5))

(event `InputAxis|InputAxis_RighLeft`
  (params (AxisValue :type "Float (single-precision)"))
  ;[0.2619 0.8901 1] move camera
  (`self.AddMovementInput` (0.0 1.0 0.0) AxisValue))

(event `self.ReceiveTick`
  (params (DeltaSeconds :type "Float (single-precision)"))
  (bind _gamemanager (`self.GameManager`))
  (bind _worldcoords_adjacent (`self.WorldCoords_Adjacent`))
  (bind _returnvalue (- (/ (`self.LoadDistance`) 1000.0) 1.0))
  (bind _returnvalue_2 (`KismetMathLibrary.Lerp` -1000.0 -5000.0 _returnvalue))
  (bind _returnvalue_3 (`KismetMathLibrary.Lerp` 1000.0 5000.0 _returnvalue))
  (bind _returnvalue_4 (`KismetMathLibrary.Vector_SnappedToGrid` (`SceneComponent.K2_GetComponentLocation` (`self.DefaultSceneRoot`)) (`KismetMathLibrary.Conv_IntToDouble` (`/Game/BaseGame/Blueprints/GameManager_BP.*TileGridSize` (`self.GameManager`)))))
  ;[1 1 1] get viewer Coords
  (`/Engine/EditorBlueprintResources/StandardMacros.IsValid` _gamemanager
    (:`Is Valid`
      (if (`/Game/BaseGame/Blueprints/GameManager_BP._worldGenerationComplete` _gamemanager)
        (`self.GetViewCursorCoords`)
        (bind _worldcoords (`self.GetWorldCoords` _returnvalue_4))
        (`KismetSystemLibrary.DrawDebugSphere` _returnvalue_4 25.0 4 (struct :`R` 1.0 :`G` 0.560092 :`B` 0.122709 :`A` 1.0) 0.01 1.0)
        (set `self.WorldCoords` _worldcoords)
        (if (`self.Possessed`)
          (`KismetArrayLibrary.Array_Clear` _worldcoords_adjacent)
          (bind _output_get (set `self._AllAjacents` (`SceneComponent.K2_GetComponentLocation` (`self.DefaultSceneRoot`))))
          (for _index (range 8)
            (if (`self.ShowAdjacent`)
              (bind _returnvalue_5 (select `int` _index :`0` (+ _output_get (`KismetMathLibrary.MakeVector` _returnvalue_3 _returnvalue_2)) :`1` (+ _output_get (`KismetMathLibrary.MakeVector` _returnvalue_3)) :`2` (+ _output_get (`KismetMathLibrary.MakeVector` _returnvalue_3 _returnvalue_3)) :`3` (+ _output_get (`KismetMathLibrary.MakeVector` 0.0 _returnvalue_3)) :`4` (+ _output_get (`KismetMathLibrary.MakeVector` _returnvalue_2 _returnvalue_3)) :`5` (+ _output_get (`KismetMathLibrary.MakeVector` _returnvalue_2)) :`6` (+ _output_get (`KismetMathLibrary.MakeVector` _returnvalue_2 _returnvalue_2)) :`7` (+ _output_get (`KismetMathLibrary.MakeVector` 0.0 _returnvalue_2))))
              (`KismetSystemLibrary.DrawDebugSphere` _returnvalue_5 100.0 12 (struct :`R` 1.0 :`G` 1.0 :`B` 1.0 :`A` 1.0) 0.01 1.0))
            (bind (_worldcoords_2 _valid) (`self.GetWorldCoords` _returnvalue_5))
            (if _valid
              (`KismetArrayLibrary.Array_Add` _worldcoords_adjacent _worldcoords_2)))
          (`self.DebugText`))))))

(fn `Debug_DrawEntityNavData`
  (params (NavData :type "/Game/BaseGame/Data/EntityNavData_Struct Structure"))
  (bind (_navindex _navstep _startcoords _goalcoords) (break `/Game/BaseGame/Data/EntityNavData_Struct` NavData))
  (bind (_x _y) (break `/Game/BaseGame/Data/WorldCoords_Struct` _goalcoords))
  (bind __tilegridsize (`/Game/BaseGame/Blueprints/GameManager_BP.*TileGridSize` (`self.GameManager`)))
  (for _array_element _navstep
    (bind (_x_2 _y_2) (`KismetMathLibrary.BreakVector2D` _array_element))
    (`KismetSystemLibrary.DrawDebugSphere` (`KismetMathLibrary.MakeVector` (* _x_2 __tilegridsize) (* _y_2 __tilegridsize)) 12.5 4 (struct :`R` 1.0 :`G` 0.300841 :`B` 0.95976 :`A` 1.0) 0.1 1.0))
  (`KismetSystemLibrary.DrawDebugSphere` (`KismetMathLibrary.MakeVector` (* _x __tilegridsize) (* _y __tilegridsize)) 25.0 6 (struct :`R` 0.593488 :`B` 1.0 :`A` 1.0) 0.1 1.0))

(fn `DebugText`
  (locals (_entityText :type String) (NewLocalVar_0 :type "Array of /Game/BaseGame/Data/EntityRefData_Struct Structure"))
  (bind __entitiesundercursor (`self._entitiesUnderCursor`))
  (bind _gamemanager (`self.GameManager`))
  (bind _worldcoords_cursor (`self.WorldCoords_Cursor`))
  (bind _gamemanager_2 (`self.GameManager`))
  (bind (_x _y _tilex _tiley _chunkx _chunky _zonex _zoney) (break `/Game/BaseGame/Data/WorldCoords_Struct` (`self.WorldCoords_Cursor`)))
  (bind (_x_2 _y_2 _tilex_2 _tiley_2 _chunkx_2 _chunky_2 _zonex_2 _zoney_2) (break `/Game/BaseGame/Data/WorldCoords_Struct` _worldcoords_cursor))
  (bind (_x_3 _y_3 _tilex_3 _tiley_3 _chunkx_3 _chunky_3 _zonex_3 _zoney_3) (break `/Game/BaseGame/Data/WorldCoords_Struct` _worldcoords_cursor))
  (bind (_x_4 _y_4 _tilex_4 _tiley_4 _chunkx_4 _chunky_4 _zonex_4 _zoney_4) (break `/Game/BaseGame/Data/WorldCoords_Struct` (`self.WorldCoords`)))
  (bind (_x_5 _y_5 _tilex_5 _tiley_5 _chunkx_5 _chunky_5 _zonex_5 _zoney_5) (break `/Game/BaseGame/Data/WorldCoords_Struct` (`self.WorldCoords_Cursor`)))
  (bind __zonesize (`/Game/BaseGame/Blueprints/GameManager_BP.*ZoneSize` _gamemanager))
  (bind __tilegridsize (`/Game/BaseGame/Blueprints/GameManager_BP.*TileGridSize` _gamemanager))
  (bind _tilemapdata (`/Game/BaseGame/Blueprints/GameManager_BP.TileMapData` _gamemanager))
  (bind _chunksperzone (`/Game/BaseGame/Blueprints/GameManager_BP.ChunksPerZone` _gamemanager))
  (bind _zonex_6 (break `/Game/BaseGame/Data/TileChunkDataArray2D_Struct` (`|GetArrayItem` _tilemapdata (`KismetMathLibrary.Clamp` _zonex_3 0 __zonesize))))
  (bind (_detailzonex _detailzoney _detailzoneid _chunkdata) (break `/Game/BaseGame/Data/TileChunkDataArray_Struct` (`|GetArrayItem` _zonex_6 (`KismetMathLibrary.Clamp` _zoney_3 0 __zonesize))))
  (bind _chunkdatay (break `/Game/BaseGame/Data/TileDataArray2D_Struct` (`|GetArrayItem` _chunkdata (`KismetMathLibrary.Clamp` _chunkx_3 0 _chunksperzone))))
  (bind (_chunkx_6 _chunky_6 _chunkid _chunktiledata _entitydataref) (break `/Game/BaseGame/Data/ChunkDataArray_Struct` (`|GetArrayItem` _chunkdatay (`KismetMathLibrary.Clamp` _chunky_3 0 _chunksperzone))))
  (bind _tilex_6 (break `/Game/BaseGame/Data/TileData_Struct` _chunktiledata))
  (bind _characterentities (break `/Game/BaseGame/Data/EntityRefArrayData_Struct` _entitydataref))
  (bind _y_6 (break `/Game/BaseGame/Data/MapData_Struct` (`|GetArrayItem` _tilex_6 (`KismetMathLibrary.Clamp` _tilex_3 0 __tilegridsize))))
  (bind _returnvalue (and (`KismetArrayLibrary.Array_IsValidIndex` _zonex_6 _zoney_2) (`KismetArrayLibrary.Array_IsValidIndex` _chunkdatay _chunky_2) (`KismetArrayLibrary.Array_IsValidIndex` _y_6 _tiley_2) (`KismetArrayLibrary.Array_IsValidIndex` _tilex_6 _tilex_2) (`KismetArrayLibrary.Array_IsValidIndex` _chunkdata _chunkx_2) (`KismetArrayLibrary.Array_IsValidIndex` _tilemapdata _zonex_2)))
  ;[1 1 1] chunk data
  (if (`self.Possessed`)
    (`KismetSystemLibrary.PrintString` "========" true true (struct :`R` 0.348958 :`G` 0.348958 :`B` 0.348958 :`A` 1.0) 0.0001)
    (`KismetSystemLibrary.PrintString` (`KismetStringLibrary.Concat_StrStr` (`KismetStringLibrary.Conv_IntToString` (`KismetArrayLibrary.Array_Length` (`/Game/BaseGame/Blueprints/GameManager_BP.LoadedChunks` _gamemanager_2))) " Chunk(s) loaded...") true true (struct :`R` 1.0 :`G` 0.958056 :`B` 0.407714 :`A` 1.0) 0.0001)
    (`KismetSystemLibrary.PrintString` (`KismetStringLibrary.Concat_StrStr` ">> Game Time : " (`KismetStringLibrary.Conv_IntToString` (`/Game/BaseGame/Blueprints/GameManager_BP.GameTime` _gamemanager_2)) " <<") true true (struct :`G` 0.04842 :`B` 1.0 :`A` 1.0) 0.0001)
    (`KismetSystemLibrary.PrintString` "========" true true (struct :`R` 0.348958 :`G` 0.348958 :`B` 0.348958 :`A` 1.0) 0.0001)
    ;[1 1 1] find entities under curosr
    (`KismetArrayLibrary.Array_Clear` (`self._entitiesUnderCursor`))
    (if _returnvalue
      (bind _output_get (set `local.NewLocalVar_0` _characterentities))
      (for _array_element _output_get
        (bind (_x_6 _y_7 _tilex_7 _tiley_6 _chunkx_7 _chunky_7 _zonex_7 _zoney_6) (break `/Game/BaseGame/Data/WorldCoords_Struct` (`.WorldCoords_5_9EA145C4446AA45B93598F9F6B1B28F6` (break `/Game/BaseGame/Data/EntityRefData_Struct` _array_element))))
        (if (and (== _tilex_7 _tilex_5) (== _tiley_6 _tiley_5) (== _chunkx_7 _chunkx_5) (== _chunky_7 _chunky_5) (== _zonex_7 _zonex_5) (== _zoney_6 _zoney_5))
          (`KismetArrayLibrary.Array_Add` (`self._entitiesUnderCursor`) _array_element)
          (bind (_loadedintochunk _index _worldcoords _visualref) (break `/Game/BaseGame/Data/EntityData_Struct` (`|GetArrayItem` (`.CharacterEntities_15_5AFF34674848CE85FA2B3C9A136CBFCF` (break `/Game/BaseGame/Data/EntityArrayData_Struct` (`/Game/BaseGame/Blueprints/GameManager_BP.EntityData` (`self.GameManager`)))) (`.Index_3_927E5EEF4BAE72947D1AAB872AE02074` (break `/Game/BaseGame/Data/EntityRefData_Struct` _array_element)))))
          (set `local._entityText` (`KismetStringLibrary.Concat_StrStr` (`local._entityText`) " \n" (`KismetStringLibrary.Concat_StrStr` "#" (`KismetStringLibrary.Conv_IntToString` _index) ", " (`KismetSystemLibrary.GetDisplayName` _visualref))))))
      ;[1 1 1] draw nav data
      (for _array_element_2 __entitiesundercursor
        (if (`KismetArrayLibrary.Array_IsValidIndex` __entitiesundercursor)
          (`self.Debug_DrawEntityNavData` (`.NavData_26_AA42227145B07B89712559B140E9CE50` (break `/Game/BaseGame/Data/EntityData_Struct` (`|GetArrayItem` (`.CharacterEntities_15_5AFF34674848CE85FA2B3C9A136CBFCF` (break `/Game/BaseGame/Data/EntityArrayData_Struct` (`/Game/BaseGame/Blueprints/GameManager_BP.EntityData` (`self.GameManager`)))) (`.Index_3_927E5EEF4BAE72947D1AAB872AE02074` (break `/Game/BaseGame/Data/EntityRefData_Struct` _array_element_2))))))
          (else
            (break)))))
    ;[1 1 1] Comment
    (if _returnvalue
      (`KismetSystemLibrary.PrintString` (`KismetStringLibrary.Concat_StrStr` "Entities : " (`local._entityText`)) true true (struct :`R` 1.0 :`G` 1.0 :`B` 1.0 :`A` 1.0) 0.0001)
      (`KismetSystemLibrary.PrintString` (`KismetStringLibrary.Concat_StrStr` (`KismetStringLibrary.Conv_IntToString` (`KismetArrayLibrary.Array_Length` _characterentities)) " Character Entities(s) In Cursor Chunk...") true true (struct :`R` 1.0 :`G` 1.0 :`B` 1.0 :`A` 1.0) 0.0001)
      (`KismetSystemLibrary.PrintString` (`KismetStringLibrary.Concat_StrStr` (`KismetStringLibrary.Conv_IntToString` (`KismetArrayLibrary.Array_Length` (`.CharacterEntities_15_5AFF34674848CE85FA2B3C9A136CBFCF` (break `/Game/BaseGame/Data/EntityArrayData_Struct` (`/Game/BaseGame/Blueprints/GameManager_BP.EntityData` (`self.GameManager`)))))) " Character Entities(s) In World...") true true (struct :`R` 1.0 :`G` 1.0 :`B` 1.0 :`A` 1.0) 0.0001)
      (`KismetSystemLibrary.PrintString` (`KismetStringLibrary.Concat_StrStr` "        ID : " (`KismetStringLibrary.Conv_IntToString` (`|GetArrayItem` _y_6 (`KismetMathLibrary.Clamp` _tiley_3 0 __tilegridsize)))) true true (struct :`R` 1.0 :`G` 1.0 :`B` 1.0 :`A` 1.0) 0.0001))
    (`KismetSystemLibrary.PrintString` (`KismetStringLibrary.Concat_StrStr` "   Zone : X - " (`KismetStringLibrary.Conv_IntToString` _zonex) ", Y - " (`KismetStringLibrary.Conv_IntToString` _zoney)) true true (struct :`R` 1.0 :`G` 1.0 :`B` 1.0 :`A` 1.0) 0.0001)
    (`KismetSystemLibrary.PrintString` (`KismetStringLibrary.Concat_StrStr` "Chunk : X - " (`KismetStringLibrary.Conv_IntToString` _chunkx) ", Y - " (`KismetStringLibrary.Conv_IntToString` _chunky)) true true (struct :`R` 1.0 :`G` 1.0 :`B` 1.0 :`A` 1.0) 0.0001)
    (`KismetSystemLibrary.PrintString` (`KismetStringLibrary.Concat_StrStr` "    Tile : X - " (`KismetStringLibrary.Conv_IntToString` _tilex) ", Y - " (`KismetStringLibrary.Conv_IntToString` _tiley)) true true (struct :`R` 1.0 :`G` 1.0 :`B` 1.0 :`A` 1.0) 0.0001)
    (`KismetSystemLibrary.PrintString` (`KismetStringLibrary.Concat_StrStr` "World : X - " (`KismetStringLibrary.Conv_IntToString` _x) ", Y - " (`KismetStringLibrary.Conv_IntToString` _y)) true true (struct :`R` 1.0 :`G` 1.0 :`B` 1.0 :`A` 1.0) 0.0001)
    (`KismetSystemLibrary.PrintString` "> CURSOR" true true (struct :`R` 1.0 :`G` 1.0 :`B` 1.0 :`A` 1.0) 0.0001)
    (`KismetSystemLibrary.PrintString` "========" true true (struct :`R` 0.348958 :`G` 0.348958 :`B` 0.348958 :`A` 1.0) 0.0001)
    ;[1 1 1] Comment
    (`KismetSystemLibrary.PrintString` (`KismetStringLibrary.Concat_StrStr` "   Zone : X - " (`KismetStringLibrary.Conv_IntToString` _zonex_4) ", Y - " (`KismetStringLibrary.Conv_IntToString` _zoney_4)) true true (struct :`R` 1.0 :`G` 1.0 :`B` 1.0 :`A` 1.0) 0.0001)
    (`KismetSystemLibrary.PrintString` (`KismetStringLibrary.Concat_StrStr` "Chunk : X - " (`KismetStringLibrary.Conv_IntToString` _chunkx_4) ", Y - " (`KismetStringLibrary.Conv_IntToString` _chunky_4)) true true (struct :`R` 1.0 :`G` 1.0 :`B` 1.0 :`A` 1.0) 0.0001)
    (`KismetSystemLibrary.PrintString` (`KismetStringLibrary.Concat_StrStr` "    Tile : X - " (`KismetStringLibrary.Conv_IntToString` _tilex_4) ", Y - " (`KismetStringLibrary.Conv_IntToString` _tiley_4)) true true (struct :`R` 1.0 :`G` 1.0 :`B` 1.0 :`A` 1.0) 0.0001)
    (`KismetSystemLibrary.PrintString` (`KismetStringLibrary.Concat_StrStr` "World : X - " (`KismetStringLibrary.Conv_IntToString` _x_4) ", Y - " (`KismetStringLibrary.Conv_IntToString` _y_4)) true true (struct :`R` 1.0 :`G` 1.0 :`B` 1.0 :`A` 1.0) 0.0001)
    (`KismetSystemLibrary.PrintString` "> VIEW" true true (struct :`R` 1.0 :`G` 1.0 :`B` 1.0 :`A` 1.0) 0.0001)))

(fn `GetViewCursorCoords`
  (bind _returnvalue (`GameplayStatics.GetPlayerController` 0))
  (bind (_locationx _locationy) (`PlayerController.GetMousePosition` _returnvalue))
  (bind (_worldlocation _worlddirection _returnvalue_2) (`PlayerController.DeprojectScreenPositionToWorld` _returnvalue _locationx _locationy))
  (bind _returnvalue_3 (`KismetMathLibrary.Vector_SnappedToGrid` _worldlocation (`KismetMathLibrary.Conv_IntToDouble` (`/Game/BaseGame/Blueprints/GameManager_BP.*TileGridSize` (`self.GameManager`)))))
  (if (`self.Possessed`)
    (if _returnvalue_2
      (`KismetSystemLibrary.DrawDebugSphere` _returnvalue_3 25.0 4 (struct :`R` 1.0 :`G` 0.747565 :`B` 0.159149 :`A` 1.0) 0.01 1.0)
      (bind (_worldcoords _valid) (`self.GetWorldCoords` _returnvalue_3))
      (if _valid
        (set `self.WorldCoords_Cursor` (`self.ClampWorldCoords` _worldcoords))))))

(fn `GetWorldCoords`
  (params (InVec :type "Vector Structure"))
  (returns (WorldCoords :type "/Game/BaseGame/Data/WorldCoords_Struct Structure") (Valid :type Boolean))
  (bind (_x _y) (`KismetMathLibrary.BreakVector3f` InVec))
  (bind _gamemanager (`self.GameManager`))
  (bind _chunksperzone (`/Game/BaseGame/Blueprints/GameManager_BP.ChunksPerZone` _gamemanager))
  (bind __zonesize (`/Game/BaseGame/Blueprints/GameManager_BP.*ZoneSize` (`self.GameManager`)))
  (bind __tilegridsize (`/Game/BaseGame/Blueprints/GameManager_BP.*TileGridSize` _gamemanager))
  (bind _returnvalue (`KismetMathLibrary.Conv_IntToDouble` (`/Game/BaseGame/Blueprints/GameManager_BP.*TileGridSize` _gamemanager)))
  (bind _returnvalue_2 (`KismetMathLibrary.Conv_IntToDouble` _chunksperzone))
  (bind _returnvalue_3 (`KismetMathLibrary.Conv_IntToDouble` (`/Game/BaseGame/Blueprints/GameManager_BP.*TIleMapSize` _gamemanager)))
  (bind _returnvalue_4 (`KismetMathLibrary.Conv_IntToDouble` (/ (* __tilegridsize (* (`/Game/BaseGame/Blueprints/GameManager_BP.*TIleMapSize` _gamemanager) (`/Game/BaseGame/Blueprints/GameManager_BP.ChunksPerZone` _gamemanager))) _chunksperzone)))
  (bind (_remainder _returnvalue_5) (`KismetMathLibrary.FMod` (/ _x _returnvalue_4) _returnvalue_2))
  (bind (_remainder_2 _returnvalue_6) (`KismetMathLibrary.FMod` (/ _y _returnvalue_4) _returnvalue_2))
  (return (make `/Game/BaseGame/Data/WorldCoords_Struct` (`KismetMathLibrary.FTrunc` (/ _x __tilegridsize)) (`KismetMathLibrary.FTrunc` (/ _y __tilegridsize)) (`KismetMathLibrary.FTrunc` (`KismetMathLibrary.FMod` (/ _x _returnvalue) _returnvalue_3)) (`KismetMathLibrary.FTrunc` (`KismetMathLibrary.FMod` (/ _y _returnvalue) _returnvalue_3)) (`KismetMathLibrary.FTrunc` _remainder) (`KismetMathLibrary.FTrunc` _remainder_2) _returnvalue_5 _returnvalue_6) (and (and (< _returnvalue_5 __zonesize) (< _returnvalue_6 __zonesize)) (and (>= _returnvalue_5 0) (>= _returnvalue_6 0)))))

(fn `Possess`
  (`Controller.Possess` (`GameplayStatics.GetPlayerController` 0) self)
  (`self.SetupPlayerControls`))

(fn `SetupPlayerControls`
  (set `PlayerController.bShowMouseCursor` true (`GameplayStatics.GetPlayerController` 0))
  (set `self._zoom` (`self.DefaultZoom`))
  (set `FloatingPawnMovement.MaxSpeed` (`self.CameraMoveSpeed`) (`self.FloatingPawnMovement`))
  (set `self.Possessed` true))

(fn `UserConstructionScript`)