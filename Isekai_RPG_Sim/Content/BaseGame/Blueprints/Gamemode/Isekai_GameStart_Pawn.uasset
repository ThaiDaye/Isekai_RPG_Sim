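; Isekai_GameStart_Pawn is the game-start pawn that bridges the player to world generation and gameplay.
; On BeginPlay it caches the GameManager_BP found in the level and shows the mouse cursor.
; StartGame tells the manager to begin generation and, as a temporary step, opens the main UI on IsekaiRPG_HUD.
; ReadyToPlay calls Possess on the manager's first game viewer.
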(event `self.ReceiveBeginPlay`
  (bind _outactors (`GameplayStatics.GetAllActorsOfClass` "/Game/BaseGame/Blueprints/GameManager_BP.GameManager_BP_C"))
  (set `self.GameManager` (`|GetArrayItem` _outactors))
  (set `PlayerController.bShowMouseCursor` true (`GameplayStatics.GetPlayerController` 0)))

(event `StartGame`
  (bind _asisekai_rpg_hud (cast `/Game/BaseGame/Blueprints/Gamemode/IsekaiRPG_HUD` (`PlayerController.GetHUD` (`GameplayStatics.GetPlayerController` 0))))
  (`/Game/BaseGame/Blueprints/GameManager_BP.BeginGeneration` (`self.GameManager`))
  ;[1 0 0] temp
  (`/Game/BaseGame/Blueprints/Gamemode/IsekaiRPG_HUD.mainUI` _asisekai_rpg_hud))

(event `ReadyToPlay`
  (`/Game/BaseGame/Blueprints/GameViewer_BP.Possess` (`|GetArrayItem` (`/Game/BaseGame/Blueprints/GameManager_BP.GameViewers` (`self.GameManager`)))))

(fn `UserConstructionScript`)