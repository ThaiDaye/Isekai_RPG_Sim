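; EntityVisual_BP is a visual actor for an entity that slides smoothly to a new location on request.
; LerpToLocation captures the current position and the target, then restarts the 1Sec timeline, whose track drives a vector lerp between them.
; Each update moves the actor without sweep and skips the move once it already sits exactly at the target.
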(event `self.ReceiveBeginPlay`)

(event `LerpToLocation`
  (params (TargetLoc :type "Vector Structure"))
  (set `self._startLoc` (`self.K2_GetActorLocation`))
  (set `self._endLoc` TargetLoc)
  (bind (_direction _newtrack_0) (`Timeline|1Sec` :!via `PlayFromStart`)
    (:`Update`
      (if (not (== (`self._endLoc`) (`self.K2_GetActorLocation`)))
        (`self.K2_SetActorLocation` (`KismetMathLibrary.VLerp` (`self._startLoc`) (`self._endLoc`) _newtrack_0))))))

(fn `UserConstructionScript`)